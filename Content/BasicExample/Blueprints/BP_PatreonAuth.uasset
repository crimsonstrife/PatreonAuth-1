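; BP_PatreonAuth is a basic example Blueprint that starts Patreon authentication through an in-game web browser.
; On BeginPlay it creates the Patreon web browser widget for the first player, adds it to the viewport and hands its browser to PatreonAuth to authenticate.
; A helper function prints a Twitch error's name, status and message, but nothing in this Blueprint calls it.
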(event EventBeginPlay
  (bind _returnvalue (UserInterface|CreateWidget "/PatreonAuth/BasicExample/UMG/WBP_WebBrowserBasicExamplePatreon.WBP_WebBrowserBasicExamplePatreon_C" (Game|GetPlayerController 0)))
  (bind _output_get (Variables|Default|SetWebBrowserWidget _returnvalue))
  (Variables|Default|SetWebBrowser (Variables|/PatreonAuth/BasicExample/UMG/WBP_WebBrowserBasicExamplePatreon.WBP_WebBrowserBasicExamplePatreon_C|GetWebBrowser_55 _output_get))
  (UserInterface|Viewport|AddtoViewport (Variables|Default|GetWebBrowserWidget) 0)
  (Class|PatreonAuthComponent|Authenticate (Variables|Default|GetPatreonAuth) (Variables|Default|GetWebBrowser)))

(fn ConstructionScript)

(fn PrintTwitchError
  (params (TwitchError :type Twitch%20Error%20Structure))
  (bind (_error _status _message) (Utilities|Struct|BreakTwitchError TwitchError))
  (Development|PrintString (Utilities|String|Append _error "(" (Utilities|String|ToString(Integer) _status) "): " _message) true true "(R=1.000000,G=0.055564,B=0.000000,A=1.000000)" 5.0))